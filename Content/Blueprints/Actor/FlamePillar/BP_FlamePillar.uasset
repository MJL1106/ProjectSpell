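; Flame pillar actor that makes its fire light flicker continuously from BeginPlay.
; It randomly picks one of two flame intensity timelines, plays it from the start, then picks again when it finishes.
; Each timeline update scales the light's base intensity by the curve value, so the random chaining varies the flicker pattern.
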(event Custom|StartTimeline_1
  (bind _flameintensity (Timeline|FlameIntensity_1 PlayFromStart)
    (:Update
      (CallFunction|ScaleFlameIntensity _flameintensity))
    (:Finished
      (CallFunction|ChooseTImeline))))

(event Custom|StartTimeline_2
  (bind _flameintensity (Timeline|FlameIntensity_2 PlayFromStart)
    (:Update
      (CallFunction|ScaleFlameIntensity _flameintensity))
    (:Finished
      (CallFunction|ChooseTImeline))))

(event Custom|ChooseTImeline
  (switch int (Math|Random|RandomIntegerinRange 0 1)
    (:Default
      (CallFunction|StartTimeline2 :!label _label))
    (:0
      (CallFunction|StartTimeline1))
    (:1
      (goto _label))))

(event EventBeginPlay
  (CallFunction|ChooseTImeline))

(fn ConstructionScript)

(fn ScaleFlameIntensity
  (params (Intensity :type Float%20%28double-precision%29))
  (Rendering|Components|Light|SetIntensity (Variables|Default|GetFireLight) (* (Variables|Default|GetBaseInensity) Intensity)))