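; Lightning Shockwave bolt actor that flies straight forward and detonates at the end of its travel distance.
; On authority, StartOutgoingTimeline lerps its location along a timeline without sweeping.
; When the timeline finishes, it calls OnHit, gathers live players within the outer damage radius, ignoring its owner.
; Each receives radial explosion damage with a death impulse pointing away from the blast, then the bolt destroys itself.
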(event EventStartOutgoingTimeline
  (bind _returnvalue (Components|GetOwner))
  (bind _self self)
  (bind _array (Utilities|Array|MakeArray _returnvalue))
  (Networking|SwitchHasAuthority
    (:Authority
      (Variables|Default|SetInitialLocation (Transformation|GetActorLocation))
      (Variables|Default|SetApexLocation (+ (Variables|Default|GetInitialLocation) (* (Transformation|GetActorForwardVector) (Variables|Default|GetTravelDistance))))
      (bind _location (Timeline|LocationTimeline Play)
        (:Update
          (Transformation|SetActorLocation (Math|Vector|Lerp(Vector) (Variables|Default|GetInitialLocation) (Variables|Default|GetApexLocation) _location) false false))
        (:Finished
          (Class|AuraProjectile|OnHit)
          (Utilities|Array|Add _array _self)
          (bind _outoverlappingactors (Class|AuraAbilitySystemLibrary|GetLivePlayersWithinRadius _self _array (Variables|Default|GetRadialDamageOuter) (Transformation|GetActorLocation)))
          (Variables|Default|SetOverlappingEnemies _outoverlappingactors)
          (Class|AuraAbilitySystemLibrary|SetIsRadialDamageEffectParam (Variables|Default|GetExplosionDamageParams) true (Variables|Default|GetRadialDamageInner) (Variables|Default|GetRadialDamageOuter) (Transformation|GetActorLocation))
          (for _array_element (Variables|Default|GetOverlappingEnemies)
            (Class|AuraAbilitySystemLibrary|SetTargetEffectParamsASC (Variables|Default|GetExplosionDamageParams) (Ability|GetAbilitySystemComponent _array_element))
            (Variables|Default|SetKnockbackDirection (- (Transformation|GetActorLocation _array_element) (Transformation|GetActorLocation)))
            (Class|AuraAbilitySystemLibrary|SetDeathImpulseDirection (Variables|Default|GetExplosionDamageParams) (Variables|Default|GetKnockbackDirection) (Variables|Default|GetDeathImpulseMagnitude))
            (Class|AuraAbilitySystemLibrary|ApplyDamageEffect (Variables|Default|GetExplosionDamageParams)))
          (Actor|DestroyActor))))))

(fn ConstructionScript)