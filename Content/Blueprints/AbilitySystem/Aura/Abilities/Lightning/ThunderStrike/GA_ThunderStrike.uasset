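; Gameplay ability that casts Thunder Strike, an area lightning attack at the location under the mouse.
; It turns the avatar toward the target, plays a cast montage and spawns the Niagara effect on the montage's gameplay event.
; If the cursor hit a player or enemy, a line trace places the effect on the floor below.
; After a short delay, the authority plays impact sound, damages nearby live players except the caster, and ends the ability.
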(event Ability|EventActivateAbility
  (bind (_returnvalue _returnvalue2 _array) (CallFunction|GetLineTraceParams))
  (Ability|CommitAbility)
  (bind _datahandle (|TargetDataUnderMouse)
    (:ValidData
      (Variables|Default|SetThunderStrikeLocation (.Location (Collision|BreakHitResult (Ability|TargetData|GetHitResultfromTargetData _datahandle))))
      (Variables|Default|SetMouseHitActor (.HitActor (Collision|BreakHitResult (Ability|TargetData|GetHitResultfromTargetData _datahandle))))
      (Class|CombatInterface|UpdateFacingTarget(Message) (Ability|GetAvatarActorfromActorInfo) (Variables|Default|GetThunderStrikeLocation))
      (|PlayMontageandWaitProxy "None" "/Game/Stylized_Wizard/Animations/CharacterAnimations/Abilities/AM_Cast_ThunderStrike.AM_Cast_ThunderStrike" 1.0 "None" false 1.0 0.0 false
        (:then
          (Ability|Tasks|WaitGameplayEvent "(TagName=\"Event.Montage.ThunderStrike\")" 0
            (:EventReceived
              (if (CallFunction|CheckHitActorImplementsInterface)
                ;[1 1 1] Mouse Hit Actor is an enemy or player so use linetrace to spawn system on ground
                (bind _outhit (Collision|LineTraceByChannel _returnvalue _returnvalue2 "TraceTypeQuery1" false _array "None"))
                (bind _output_get (Variables|Default|SetFloorHitLocation (.ImpactPoint (Collision|BreakHitResult _outhit))))
                (Niagara|SpawnSystematLocation "/Game/Blueprints/AbilitySystem/Aura/Abilities/Lightning/ThunderStrike/NS_LightningAEO_White.NS_LightningAEO_White" _output_get)
                (else
                  (Niagara|SpawnSystematLocation "/Game/Blueprints/AbilitySystem/Aura/Abilities/Lightning/ThunderStrike/NS_LightningAEO_White.NS_LightningAEO_White" (Variables|Default|GetThunderStrikeLocation))))
              (Ability|HasAuthority
                (:True
                  (Utilities|FlowControl|Delay 0.65)
                  (Audio|PlaySoundatLocation "/Game/Assets/Sounds/Abilities/ThunderStrike/sfx_ThunderStrike_Impact.sfx_ThunderStrike_Impact" (Variables|Default|GetThunderStrikeLocation) "0, 0, 0" 1.0 1.0 0.0 0 0 0 0)
                  (CallFunction|DealDamagetoPlayersinRadius (Variables|Default|GetThunderStrikeLocation)))))))))))

(fn DealDamagetoPlayersinRadius
  (params (SphereOrigin :type Vector%20%28by%20ref%29))
  (bind _outoverlappingactors (Class|AuraAbilitySystemLibrary|GetLivePlayersWithinRadius (Ability|GetAvatarActorfromActorInfo) (Utilities|Array|MakeArray (Ability|GetAvatarActorfromActorInfo)) 2.4e+02 SphereOrigin))
  ;[1 1 1] If 0 then no players to damage
  (if (> (Utilities|Array|Length _outoverlappingactors) 0)
    (for _array_element _outoverlappingactors
      (Class|AuraAbilitySystemLibrary|ApplyDamageEffect (Class|AuraDamageGameplayAbility|MakeDamageEffectParamsfromClassDefaults _array_element "0, 0, 0" false "0, 0, 0" false "0, 0, 0" false 0.0)))
    (Ability|EndAbility)
    (else
      (Ability|EndAbility))))

(fn CheckHitActorImplementsInterface
  (bind _mousehitactor (Variables|Default|GetMouseHitActor))
  (return (or (Utilities|DoesObjectImplementInterface _mousehitactor "/Script/Aura.PlayerInterface") (Utilities|DoesObjectImplementInterface _mousehitactor "/Script/Aura.EnemyInterface"))))

(fn GetLineTraceParams
  (bind _mousehitactor (Variables|Default|GetMouseHitActor))
  (return (Transformation|GetActorLocation _mousehitactor) (- (Variables|Default|GetThunderStrikeLocation) "0.000000,0.000000,300.000000") (Utilities|Array|MakeArray (Ability|GetAvatarActorfromActorInfo) _mousehitactor)))