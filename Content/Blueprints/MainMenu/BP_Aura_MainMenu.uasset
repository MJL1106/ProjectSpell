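; BP_Aura_MainMenu drives the main menu scene, bringing up the menu UI and animating its decorative fireball and magic circle.
; BeginPlay adds WBP_MainMenu to the viewport, switches to UI-only input and shows the cursor.
; Tick bobs the fireball vertically on a sine of a wrapped time counter and spins the decal at a set rate.
; The menu music spawn is disconnected, so it never plays.
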(event EventBeginPlay
  (bind _returnvalue (Game|GetPlayerController 0))
  (Variables|Default|SetFireballInitialLocation (Transformation|GetWorldLocation (Variables|Default|GetFIreBall)))
  (bind _returnvalue_2 (UserInterface|CreateWidget "/Game/Blueprints/UI/MainMenu/WBP_MainMenu.WBP_MainMenu_C"))
  (UserInterface|Viewport|AddtoViewport _returnvalue_2 0)
  (Input|SetInputModeUIOnly _returnvalue _returnvalue_2 "DoNotLock" false)
  (Variables|/Script/Engine.PlayerController|SetbShowMouseCursor _returnvalue true))

(event EventTick
  (params (DeltaSeconds :type Float%20%28single-precision%29))
  (CallFunction|UpdateTIme DeltaSeconds)
  (Transformation|SetWorldLocation (Variables|Default|GetFIreBall) (+ (Variables|Default|GetFireballInitialLocation) (Math|Vector|MakeVector 0.0 0.0 (CallFunction|SinTime))) false false)
  (Transformation|AddLocalRotation (Variables|Default|GetDecal) (Math|Rotator|MakeRotator (* (Utilities|Time|GetWorldDeltaSeconds) (Variables|Default|GetMagicCircleRotRate)) 0.0 0.0) false false))

(fn ConstructionScript)

(fn UpdateTIme
  (params (A :type Float%20%28double-precision%29))
  (bind _output_get (Variables|Default|SetTime (+ A (Variables|Default|GetTime))))
  (if (> _output_get 6.28318)
    (Variables|Default|SetTime 0.0)))

(fn SinTime
  (return (* (Math|Trig|Sin(Radians) (Variables|Default|GetTime)) (Variables|Default|GetAmplitude))))