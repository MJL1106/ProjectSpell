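; BP_VFXSpawner is an actor that repeatedly spawns a configurable Niagara effect and displays its name, apparently for showcasing VFX.
; One second after BeginPlay it plays the effect, then a looping timer replays it every FireRate seconds.
; Each spawn uses the Arrow component's world location and rotation.
; The construction script writes VFXName to a TextRender label.
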(event Custom|PlayVFX
  (bind _arrow (Variables|Default|GetArrow))
  (Niagara|SpawnSystematLocation (Variables|Default|GetVFX) (Transformation|GetWorldLocation _arrow) (Transformation|GetWorldRotation _arrow)))

(event EventBeginPlay
  (Utilities|FlowControl|Delay 1.0)
  (CallFunction|PlayVFX)
  (Utilities|Time|SetTimerbyEvent (delegate Custom|PlayVFX) (Variables|Default|GetFireRate) true))

(fn ConstructionScript
  (Rendering|Components|TextRender|SetText (Variables|Default|GetTextRender) (Variables|Default|GetVFX_Name)))